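; BP_Moon is a world actor for the moon, aimed and sized when constructed.
; Its construction script rotates the actor so its X axis points toward the VectorMoon location and scales it uniformly by ScaleMoon.
; Two events, SetVisibleTrue and SetVisibleFalse, show or hide the root scene component without propagating the change to child components.
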(event `Set Visible True`
  (`SceneComponent.SetVisibility` (`self.DefaultSceneRoot`) true false))

(event `Set Visible False`
  (`SceneComponent.SetVisibility` (`self.DefaultSceneRoot`) false false))

(fn `UserConstructionScript`
  (bind _scalemoon (`self.ScaleMoon`))
  (`self.K2_SetActorRotation` (`KismetMathLibrary.Conv_VectorToRotator` (`KismetMathLibrary.Normal` (- (`self.VectorMoon`) (`self.K2_GetActorLocation`)))))
  (`self.SetActorScale3D` (`KismetMathLibrary.MakeVector` _scalemoon _scalemoon _scalemoon)))