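; Actor component that makes its owning actor an interactable object with a detection volume and a named prompt.
; On BeginPlay it adds a box sized by Extents that blocks only GameTraceChannel1, plus a hidden screen-space widget component showing WB_InteractionWidget with InteractionName.
; ShowInteractionWidget toggles the prompt's visibility, and OnInterected fires the interaction through CallOnInterected.
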(event `self.ReceiveBeginPlay`
  (set `self.Owner` (`self.GetOwner`))
  (`self.AddInteractionBox`)
  (`self.AddWidget`))

(fn `AddInteractionBox`
  (bind _returnvalue (`|AddComponentByClass` :`self` (`self.Owner`) :`Class` "/Script/Engine.BoxComponent"))
  (set `self.BoxCollision` _returnvalue)
  (`BoxComponent.SetBoxExtent` _returnvalue (`self.Extents`) true)
  (`PrimitiveComponent.SetCollisionResponseToAllChannels` (`self.BoxCollision`) "ECR_Ignore")
  (`PrimitiveComponent.SetCollisionResponseToChannel` (`self.BoxCollision`) "ECC_GameTraceChannel1" "ECR_Block"))

(fn `AddWidget`
  (bind _returnvalue (`|AddComponentByClass` :`self` (`self.Owner`) :`Class` "/Script/UMG.WidgetComponent"))
  (`SceneComponent.K2_SetRelativeLocation` _returnvalue (`self.InteractionWidgetLocation`) false false)
  (`WidgetComponent.SetWidgetSpace` _returnvalue "Screen")
  (`SceneComponent.SetVisibility` _returnvalue false false)
  (bind _output_get (set `self.InteractionWidget` _returnvalue))
  (bind _returnvalue_2 (`|CreateWidget` "/Game/Interaction/WB_InteractionWidget.WB_InteractionWidget_C" null (`self.InteractionName`)))
  (`WidgetComponent.SetWidget` _output_get _returnvalue_2))

(fn `OnInterected`
  (`self.On Interected`))

(fn `ShowInteractionWidget`
  (params (`Show?` :type Boolean))
  (`SceneComponent.SetVisibility` (`self.InteractionWidget`) `Show?` false))