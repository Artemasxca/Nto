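; BP_Entity1 is an entity that pursues the player's ThirdPersonCharacter until the flashlight banishes it.
; BeginPlay prints a debug string and sets EntityOnLevel on Main_GameInstance to 1.
; Each Tick looks up the character, destroys the entity and zeroes EntityOnLevel when FlashLightActive and FlashLightEntity are both true.
; Tick also rotates it to face the player and, through a short Delay, issues AIMoveTo toward them.
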(event `self.ReceiveBeginPlay`
  (`KismetSystemLibrary.PrintString` "opopo")
  (bind _asmain_game_instance (cast `/Game/ThirdPersonBP/Warning/Main_GameInstance` (`GameplayStatics.GetGameInstance`)))
  (set `self.Main Game Instance Ref` _asmain_game_instance)
  (set `/Game/ThirdPersonBP/Warning/Main_GameInstance.Entity On Level` 1 (`self.Main Game Instance Ref`)))

(event `self.ReceiveTick`
  (params (DeltaSeconds :type "Float (single-precision)"))
  (bind _third_person_ref (`self.Third person ref`))
  (`|ExecutionSequence`
    (:`then_0`
      (bind _returnvalue (`GameplayStatics.GetActorOfClass` "/Game/ThirdPersonBP/Blueprints/ThirdPersonCharacter.ThirdPersonCharacter_C"))
      (bind _output_get (set `self.Third person ref` _returnvalue))
      (`/Engine/EditorBlueprintResources/StandardMacros.IsValid` _output_get
        (:`Is Valid`
          (if (`/Game/ThirdPersonBP/Blueprints/ThirdPersonCharacter.FlashLightActive` _returnvalue)
            (if (`/Game/ThirdPersonBP/Blueprints/ThirdPersonCharacter.FlashLightEntity` _returnvalue)
              (`self.K2_DestroyActor`)
              (set `/Game/ThirdPersonBP/Warning/Main_GameInstance.Entity On Level` 0 (`self.Main Game Instance Ref`)))))))
    (:`then_1`
      (`self.Look`))
    (:`then_2`
      (`KismetSystemLibrary.Delay` 0.2)
      (`/Engine/EditorBlueprintResources/StandardMacros.IsValid` _third_person_ref
        (:`Is Valid`
          (`|AIMoveTo` null (5.0 5.0 5.0) _third_person_ref))))))

(fn `Look`
  (bind _third_person_ref (`self.Third person ref`))
  (`/Engine/EditorBlueprintResources/StandardMacros.IsValid` _third_person_ref
    (:`Is Valid`
      (`self.K2_SetActorRotation` (`KismetMathLibrary.FindLookAtRotation` (`self.K2_GetActorLocation`) (`self.K2_GetActorLocation` _third_person_ref))))))

(fn `UserConstructionScript`)