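; BP_EntitySpawn is a spawner actor that places a single BPC_Entity in the level when its location is out of the player's view.
; Each Tick it reads EntityOnLevel and EntitySpawn from Main_GameInstance, spawning only if ProjectWorldToScreen fails for the actor's location.
; The spawn point is random within the Box bounds, centred on the Box's relative location.
; Spawning updates both GameInstance variables to block further spawns, and debug prints remain.
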(event `self.ReceiveTick`
  (params (DeltaSeconds :type "Float (single-precision)"))
  (bind _box (`self.Box`))
  (bind _main_game_instance (`self.Main Game Instance`))
  (bind _asmain_game_instance (cast `/Game/ThirdPersonBP/Warning/Main_GameInstance` (`GameplayStatics.GetGameInstance`))
    (:`then`
      (bind _output_get (set `self.Main Game Instance` _asmain_game_instance))
      (if (== (`/Game/ThirdPersonBP/Warning/Main_GameInstance.Entity On Level` (`self.Main Game Instance`)) 0)
        (if (`/Game/ThirdPersonBP/Warning/Main_GameInstance.Entity Spawn` _output_get)
          (if (`.ReturnValue` (`GameplayStatics.ProjectWorldToScreen` (`GameplayStatics.GetPlayerController` 0) (`self.K2_GetActorLocation`)))
            (`KismetSystemLibrary.PrintString` "what")
            (else
              (`|SpawnActorFromClass` "/Game/Asset/Geometry/BP_Meshes/Entity/BPC_Entity.BPC_Entity_C" (`KismetMathLibrary.MakeTransform` (`KismetMathLibrary.RandomPointInBoundingBox` (`SceneComponent.RelativeLocation` _box) (`BoxComponent.BoxExtent` _box))) "Undefined" "OverrideRootScale" null null)
              (set `/Game/ThirdPersonBP/Warning/Main_GameInstance.Entity Spawn` false _main_game_instance)
              (set `/Game/ThirdPersonBP/Warning/Main_GameInstance.Entity On Level` 1 _main_game_instance)
              (`KismetSystemLibrary.PrintString` "1111111"))))))
    (:`CastFailed`
      (`KismetSystemLibrary.PrintString` "Fail"))))

(fn `UserConstructionScript`)