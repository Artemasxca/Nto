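; BPC_Entity is an entity actor that removes itself when the player's flashlight catches it, as signalled by flags on ThirdPersonCharacter.
; On BeginPlay it caches a reference to Main_GameInstance.
; Each Tick it looks up the character with GetActorOfClass and polls FlashLightActive and FlashLightEntity.
; When both are true, it destroys itself and resets the game instance's EntityOnLevel to zero.
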(event `self.ReceiveBeginPlay`
  (bind _asmain_game_instance (cast `/Game/ThirdPersonBP/Warning/Main_GameInstance` (`GameplayStatics.GetGameInstance`)))
  (set `self.Main Game Instance Ref` _asmain_game_instance))

(event `self.ReceiveTick`
  (params (DeltaSeconds :type "Float (single-precision)"))
  (bind _returnvalue (`GameplayStatics.GetActorOfClass` "/Game/ThirdPersonBP/Blueprints/ThirdPersonCharacter.ThirdPersonCharacter_C"))
  (`/Engine/EditorBlueprintResources/StandardMacros.IsValid` _returnvalue
    (:`Is Valid`
      (if (`/Game/ThirdPersonBP/Blueprints/ThirdPersonCharacter.FlashLightActive` _returnvalue)
        (if (`/Game/ThirdPersonBP/Blueprints/ThirdPersonCharacter.FlashLightEntity` _returnvalue)
          (`self.Destroy Actor`))))))

(event `Destroy Actor`
  (`self.K2_DestroyActor`)
  (set `/Game/ThirdPersonBP/Warning/Main_GameInstance.Entity On Level` 0 (`self.Main Game Instance Ref`)))

(fn `UserConstructionScript`)