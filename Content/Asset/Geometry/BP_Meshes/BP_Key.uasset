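; BP_Key is an interactable key actor, apparently an unfinished inventory pickup.
; It caches the HUD on BeginPlay; on interaction through BPC_InteractableObject, it fetches ThirdPersonCharacter and checks CanPickUp.
; The following loop has unconnected inputs and an empty branch, leaving only debug prints.
; Disconnected logic would put a battery icon in a HUD slot, update the inventory and destroy the actor.
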(event `self.ReceiveBeginPlay`
  (bind _returnvalue (`GameplayStatics.GetActorOfClass` "/Script/Engine.HUD"))
  (set `self.Hud_Ref` _returnvalue))

(event `self.BPC_InteractableObject.On Interacted`
  (bind _returnvalue (`GameplayStatics.GetActorOfClass` "/Game/ThirdPersonBP/Blueprints/ThirdPersonCharacter.ThirdPersonCharacter_C"))
  (bind _output_get (set `self.Third Person Ref` _returnvalue))
  (`/Engine/EditorBlueprintResources/StandardMacros.IsValid` _output_get
    (:`Is Valid`
      (if (`/Game/ThirdPersonBP/Blueprints/ThirdPersonCharacter.Can Pick Up` (`self.Third Person Ref`))
        (for (_array_element _array_index) _
          (if (== _array_element null)
            _))
        (`KismetSystemLibrary.PrintString` "1")))
    (:`Is Not Valid`
      (`KismetSystemLibrary.PrintString` "1"))))

(fn `UserConstructionScript`)