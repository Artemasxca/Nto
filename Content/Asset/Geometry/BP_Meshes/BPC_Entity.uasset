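; BPC_Entity is an entity actor that disappears when the player's flashlight catches it.
; BeginPlay caches the Main_GameInstance.
; Each Tick looks up the ThirdPersonCharacter, and when both its FlashLightActive and FlashLightEntity flags are true, the entity destroys itself and resets EntityOnLevel on the game instance to zero.
; The overlap events are empty, and older overlap-style destroy chains remain disconnected.
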(event `self.ReceiveBeginPlay`
  (bind _asmain_game_instance (cast `/Game/ThirdPersonBP/Warning/Main_GameInstance` (`GameplayStatics.GetGameInstance`)))
  (set `self.Main Game Instance Ref` _asmain_game_instance))

(event `self.ReceiveTick`
  (params (DeltaSeconds :type "Float (single-precision)"))
  (bind _returnvalue (`GameplayStatics.GetActorOfClass` "/Game/ThirdPersonBP/Blueprints/ThirdPersonCharacter.ThirdPersonCharacter_C"))
  (bind _output_get (set `self.Third Person Ref` _returnvalue))
  (`/Engine/EditorBlueprintResources/StandardMacros.IsValid` _output_get
    (:`Is Valid`
      (if (`/Game/ThirdPersonBP/Blueprints/ThirdPersonCharacter.FlashLightActive` _returnvalue)
        (if (`/Game/ThirdPersonBP/Blueprints/ThirdPersonCharacter.FlashLightEntity` _returnvalue)
          (`self.K2_DestroyActor`)
          (set `/Game/ThirdPersonBP/Warning/Main_GameInstance.Entity On Level` 0 (`self.Main Game Instance Ref`)))))))

(event `self.Box.OnComponentBeginOverlap`
  (params (OverlappedComponent :type "PrimitiveComponent Object Reference") (OtherActor :type "Actor Object Reference") (OtherComp :type "PrimitiveComponent Object Reference") (OtherBodyIndex :type Integer) (bFromSweep :type Boolean) (SweepResult :type "HitResult Structure (by ref)")))

(event `self.ReceiveActorBeginOverlap`
  (params (OtherActor :type "Actor Object Reference")))

(fn `UserConstructionScript`)