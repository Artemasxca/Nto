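; BP_MasterItem is a data-driven pickup item that adds itself to the player's inventory when interacted with.
; DataFromObject validates the selected data table row and supplies the item data; BeginPlay uses it to async-load the static mesh, or destroys the actor on failure.
; On interaction, it writes itself into the first empty ThirdPersonCharacter inventory slot, sends its texture to the HUD, sets the Oil flag and destroys itself.
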(event `self.ReceiveBeginPlay`
  (bind (_dataitems _noterrors) (`self.DataFromObject`))
  (if _noterrors
    (bind _object (`|LoadAsset` (`.StaticMesh_13_13B8EE14470E562E3170579F6ACBECF8` (break `/Game/Asset/Inventory/BP_Item_Structure` _dataitems)))
      (:`Completed`
        (bind _asstatic_mesh (cast `StaticMesh` _object))
        (`StaticMeshComponent.SetStaticMesh` (`self.StaticMesh`) _asstatic_mesh)))
    (else
      (`self.K2_DestroyActor`))))

(event `self.ReceiveTick`
  (params (DeltaSeconds :type "Float (single-precision)")))

(event `BreakLoop`
  (goto _label :!via `Break`))

(event `self.BPC_InteractableObject.On Interacted`
  (bind _returnvalue (`GameplayStatics.GetActorOfClass` "/Game/ThirdPersonBP/Blueprints/ThirdPersonCharacter.ThirdPersonCharacter_C"))
  (bind _output_get (set `self.Third Person Ref` _returnvalue))
  (`/Engine/EditorBlueprintResources/StandardMacros.IsValid` _output_get
    (:`Is Valid`
      (for (_array_element _array_index) (`/Game/ThirdPersonBP/Blueprints/ThirdPersonCharacter.Inventory Array` (`self.Third Person Ref`)) :!label _label
        (if (not (!= _array_element null))
          (`KismetArrayLibrary.Array_Set` (`/Game/ThirdPersonBP/Blueprints/ThirdPersonCharacter.Inventory Array` (`self.Third Person Ref`)) _array_index self)
          (bind (_dataitems _noterrors _texture) (`self.DataFromObject`))
          (`/Game/Widget/Hud/WBP_Hud.Event Initialization Slot` (`/Game/ThirdPersonBP/Blueprints/ThirdPersonCharacter.WBP HUD Ref` (`self.Third Person Ref`)) _texture _array_index)
          (`self.BreakLoop`)
          (set `/Game/ThirdPersonBP/Blueprints/ThirdPersonCharacter.Oil` true (`self.Third Person Ref`))
          (`self.K2_DestroyActor`))))))

(fn `DataFromObject`
  (returns (DataItems :type "/Game/Asset/Inventory/BP_Item_Structure Structure") (NotErrors :type Boolean) (Texture :type "Texture2D Soft Object Reference"))
  (locals (LocalDataTable :type "DataTable Object Reference" :default "DataTable'/Game/Asset/Inventory/DT_Item.DT_Item'") (`Local Row Table` :type Name))
  (bind (_selectsubjects_datatable _selectsubjects_rowname) (break `DataTableRowHandle` (`self.SelectSubjects`)))
  (set `local.LocalDataTable` _selectsubjects_datatable)
  (set `local.Local Row Table` _selectsubjects_rowname)
  (`/Engine/EditorBlueprintResources/StandardMacros.IsValid` (`local.LocalDataTable`)
    (:`Is Valid`
      (if (not (== (`local.Local Row Table`) "None"))
        (bind _returnvalue (`|GetDataTableRow` (`local.LocalDataTable`) (`local.Local Row Table`))
          (:`then`
            (return _returnvalue true (`.Texture_10_06128CB34652876D4661798FECB69DB7` (break `/Game/Asset/Inventory/BP_Item_Structure` _returnvalue))))
          (:`RowNotFound`
            (return (struct) false null)))
        (else
          (`KismetSystemLibrary.PrintString` "Не выбран тип предмета")
          (return (struct) false null))))
    (:`Is Not Valid`
      (`KismetSystemLibrary.PrintString` "Таблица данных не выбрана" true true (struct :`G` 0.66 :`B` 1.0 :`A` 1.0) 40.0)
      (return (struct) false null))))

(fn `UserConstructionScript`)