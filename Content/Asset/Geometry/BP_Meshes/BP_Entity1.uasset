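; BP_Entity1 is an entity actor that the player's flashlight can remove from the world.
; Each tick it looks up the ThirdPersonCharacter and destroys itself when both FlashLightActive and FlashLightEntity are true.
; BeginPlay prints a debug string, and the Spawn event is empty.
; Disconnected logic would spawn another BP_Entity1 at a random point in the player's SpawnBox and clear the spawn flags, but it never runs.
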(event `self.ReceiveBeginPlay`
  (`KismetSystemLibrary.PrintString` "opopo"))

(event `Spawn`)

(event `self.ReceiveTick`
  (params (DeltaSeconds :type "Float (single-precision)"))
  (bind _returnvalue (`GameplayStatics.GetActorOfClass` "/Game/ThirdPersonBP/Blueprints/ThirdPersonCharacter.ThirdPersonCharacter_C"))
  (bind _output_get (set `self.Third person ref` _returnvalue))
  (`/Engine/EditorBlueprintResources/StandardMacros.IsValid` _output_get
    (:`Is Valid`
      (if (`/Game/ThirdPersonBP/Blueprints/ThirdPersonCharacter.FlashLightActive` _returnvalue)
        (if (`/Game/ThirdPersonBP/Blueprints/ThirdPersonCharacter.FlashLightEntity` _returnvalue)
          (`self.K2_DestroyActor`))))))

(fn `UserConstructionScript`)