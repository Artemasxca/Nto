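; Interactable car actor that acts as the finish point once the player has oil.
; Its box overlap clears the ThirdPersonCharacter's OutHot flag on entry and sets it again on exit.
; On interaction it checks the character's Oil flag, either opening the finish widget with UI-only input or playing the HUD's oil animation.
; A DoOnce gate resets after a delay only when oil is missing, throttling repeat attempts.
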(event `self.Box.OnComponentBeginOverlap`
  (params (OverlappedComponent :type "PrimitiveComponent Object Reference") (OtherActor :type "Actor Object Reference") (OtherComp :type "PrimitiveComponent Object Reference") (OtherBodyIndex :type Integer) (bFromSweep :type Boolean) (SweepResult :type "HitResult Structure (by ref)"))
  (bind _asthird_person_character (cast `/Game/ThirdPersonBP/Blueprints/ThirdPersonCharacter` OtherActor))
  (set `/Game/ThirdPersonBP/Blueprints/ThirdPersonCharacter.OutHot` false _asthird_person_character))

(event `self.Box.OnComponentEndOverlap`
  (params (OverlappedComponent :type "PrimitiveComponent Object Reference") (OtherActor :type "Actor Object Reference") (OtherComp :type "PrimitiveComponent Object Reference") (OtherBodyIndex :type Integer))
  (bind _asthird_person_character (cast `/Game/ThirdPersonBP/Blueprints/ThirdPersonCharacter` OtherActor))
  (set `/Game/ThirdPersonBP/Blueprints/ThirdPersonCharacter.OutHot` true _asthird_person_character))

(event `self.BPC_InteractableObject.On Interacted`
  (`/Engine/EditorBlueprintResources/StandardMacros.DoOnce` false :!label _label
    (:`Completed`
      (bind _returnvalue (`GameplayStatics.GetActorOfClass` "/Game/ThirdPersonBP/Blueprints/ThirdPersonCharacter.ThirdPersonCharacter_C"))
      (bind _output_get (set `self.Third Person Character ref` _returnvalue))
      (`/Engine/EditorBlueprintResources/StandardMacros.IsValid` _output_get
        (:`Is Valid`
          (if (`/Game/ThirdPersonBP/Blueprints/ThirdPersonCharacter.Oil` _returnvalue)
            (set `PlayerController.bShowMouseCursor` true (`GameplayStatics.GetPlayerController` 0))
            (`WidgetBlueprintLibrary.SetInputMode_UIOnlyEx` (`GameplayStatics.GetPlayerController` 0) null)
            (bind _returnvalue_2 (`|CreateWidget` "/Game/Widget/Hud/WBP_Finish.WBP_Finish_C"))
            (`UserWidget.AddToViewport` _returnvalue_2 0)
            (else
              (`/Game/Widget/Hud/WBP_Hud.Oil Anim` (`/Game/ThirdPersonBP/Blueprints/ThirdPersonCharacter.WBP HUD Ref` (`self.Third Person Character ref`)))
              (`KismetSystemLibrary.Delay` 6.0)
              (goto _label :!via `Reset`))))))))

(fn `UserConstructionScript`)